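; BP_TargetSpawner spawns a one-time batch of BP_Target actors when its Trigger actor is first overlapped.
; On BeginPlay it binds to the Trigger's begin-overlap event, which accepts any actor and uses a Spawned flag to block repeat batches.
; A loop places ten targets at random-direction offsets scaled by SpawnRadius around the spawner, clamping world height to a fixed band and ignoring collisions.
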(event `self.ReceiveBeginPlay`
  (set `self.Spawned` false)
  (add `self.OnActorBeginOverlap` (`self.Trigger`) (delegate `OnActorBeginOverlap_Event`)))

(event `OnActorBeginOverlap_Event` :!signature `self.OnActorBeginOverlap`
  (params (OverlappedActor :type "Actor Object Reference") (OtherActor :type "Actor Object Reference"))
  (if (not (`self.Spawned`))
    (for _ (range 1 11)
      (set `self.Spawned` true)
      (`|SpawnActorFromClass` "/Game/BP_Target.BP_Target_C" (`KismetMathLibrary.MakeTransform` (`KismetMathLibrary.MakeVector` (.x (+ (`self.K2_GetActorLocation`) (* (`KismetMathLibrary.RandomUnitVector`) (`self.Spawn Radius`)))) (.y (+ (`self.K2_GetActorLocation`) (* (`KismetMathLibrary.RandomUnitVector`) (`self.Spawn Radius`)))) (`KismetMathLibrary.FClamp` (.z (+ (`self.K2_GetActorLocation`) (* (`KismetMathLibrary.RandomUnitVector`) (`self.Spawn Radius`)))) 700.0 1200.0))) "AlwaysSpawn" "MultiplyWithRoot" null null))))

(fn `UserConstructionScript`)