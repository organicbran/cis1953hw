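; Reusable health component that tracks an owning actor's health and reports its death.
; Health starts at MaxHealth on BeginPlay, and the Damage and Heal functions adjust it, clamped between zero and the maximum.
; When Damage leaves Health at zero, it calls OnDeathMessage on the owner, leaving the death response to that actor.
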(event `self.ReceiveBeginPlay`
  (set `self.Health` (`self.Max Health`)))

(fn `Damage`
  (params (`Damage Taken` :type Integer))
  (bind _output_get (set `self.Health` (`KismetMathLibrary.Clamp` (- (`self.Health`) `Damage Taken`) 0 (`self.Max Health`))))
  (if (== _output_get 0)
    (message `/Game/BPI_Character.On Death` (`self.GetOwner`))
    (return)))

(fn `Heal`
  (params (`Damage Healed` :type Integer))
  (set `self.Health` (`KismetMathLibrary.Clamp` (+ `Damage Healed` (`self.Health`)) 0 (`self.Max Health`))))