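; BP_PatrolRoute is a patrol route for NPCs, defined by the points of a spline.
; GetPointLocation returns the world location of the current spline point.
; IncrementSplineIndex steps that index by Direction and flips Direction at the first or last point, so the route runs back and forth rather than looping.
; The event graph and construction script are empty, leaving advancement to external callers.
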(fn `Get Point Location`
  (returns (Location :type "Vector Structure"))
  (return (`SplineComponent.GetLocationAtSplinePoint` (`self.Spline`) (`self.Spline Point Index`) "World")))

(fn `Increment Spline Index`
  (bind _output_get (set `self.Spline Point Index` (+ (`self.Spline Point Index`) (`self.Direction`))))
  (if (or (== _output_get 0) (== _output_get (- (`SplineComponent.GetNumberOfSplinePoints` (`self.Spline`)) 1)))
    (set `self.Direction` (* (`self.Direction`) -1))))

(fn `UserConstructionScript`)